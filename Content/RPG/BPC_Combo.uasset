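; Actor component that drives chained melee attack combos by playing montages on its owning Character, cached at BeginPlay.
; StartAttack plays the first montage or, if an attack is already running, buffers the input as a saved attack.
; ComboAttack consumes that buffered input to play the next montage in the array, wrapping the index, at the melee speed rate.
; ResetCombo clears the attack state and returns the sequence to the start.
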(event EventBeginPlay
  (bind _ascharacter (Utilities|Casting|CastToCharacter (Components|GetOwner))
    (:then
      (Variables|Internal|SetAnimationTarget _ascharacter))
    (:CastFailed
      (Development|PrintString "WRONG ACTOR" true true "(R=1.000000,G=0.000000,B=0.000000,A=1.000000)" 1e+01))))

(event EventTick
  (params (DeltaSeconds :type Float%20%28single-precision%29)))

(fn StartAttack
  (if (Variables|Internal|GetIsAttacking)
    (Variables|Internal|SetSaveAttack true)
    (else
      (Variables|Internal|SetIsAttacking true)
      (CallFunction|PlayAttack)))
  (return))

(fn ComboAttack
  (if (Variables|Internal|GetSaveAttack)
    (Variables|Internal|SetSaveAttack false)
    (CallFunction|PlayAttack))
  (return))

(fn ResetCombo
  (Variables|Internal|SetSaveAttack false)
  (Variables|Internal|SetIsAttacking false)
  (Variables|Internal|SetCurrentCombo 0))

(fn NextComboIndex
  (LocalVariables|SetPreviousCombo (Variables|Internal|GetCurrentCombo))
  (bind _result (Math|Integer|IncrementInt (Variables|Internal|GetCurrentCombo))
    (:%20%20
      (bind _output_get (Variables|Internal|SetCurrentCombo _result))
      (if (< _output_get (Utilities|Array|Length (Variables|Combo|GetMontages)))
        _
        (else
          (Variables|Internal|SetCurrentCombo 0)))
      (return (LocalVariables|GetPreviousCombo)))))

(fn PlayAttack
  (bind _comboindex (CallFunction|NextComboIndex))
  (Animation|PlayAnimMontage (Variables|Internal|GetAnimationTarget) (Utilities|Array|Get(acopy) (Variables|Combo|GetMontages) _comboindex) (Variables|Combo|GetMeleeSpeed) "None")
  (return))